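; Horror Engine game instance that keeps user settings and audio mix state in a BP_SaveSTP save object.
; Settings load lazily or are created if absent; saving also records the current slot as the latest save.
; Master volume and music/SFX toggles update sound-class overrides and settings, using a near-zero floor instead of silence.
; Load-time init overrides only Master, fixed at that floor; music and SFX init is disconnected.
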(fn `GetUserSettings`
  (returns (UserSettings :type "Object Object Reference"))
  (bind _usersettings (`self.UserSettings`)
    (:`then`
      (return _usersettings))
    (:`else`
      (`self.LoadUserSettings`)
      (return (`self.UserSettings`)))))

(fn `InitAudioMixSettings`
  (`GameplayStatics.SetSoundMixClassOverride` "/Game/Menu/SFX/SoundMix_Master.SoundMix_Master" "/Game/Menu/SFX/SoundClass_Master.SoundClass_Master" (`KismetMathLibrary.SelectFloat` (`.Master_6_5C15BA8347FB14327EF9EE9156A9D623` (break `/Game/Menu/S_AudioMix` (`/Game/BP_SaveSTP.AudioMixer` (`self.UserSettings`)))) 0.001) 1.0 0.0))

(fn `InitUserSettings`
  (`self.InitAudioMixSettings`))

(fn `LoadUserSettings`
  (bind _returnvalue (`GameplayStatics.DoesSaveGameExist` (`self.UserSettingsSlot`)))
  (if _returnvalue
    (bind _returnvalue_2 (`GameplayStatics.LoadGameFromSlot` (`self.UserSettingsSlot`)))
    (bind _asbp_save_stp (cast `/Game/BP_SaveSTP` _returnvalue_2)
      (:`then`
        (set `self.UserSettings` _asbp_save_stp)
        (`self.InitUserSettings` :!label _label)
        (return))
      (:`CastFailed`
        (`KismetSystemLibrary.PrintString` "Cast to Save Object failed" true true (struct :`R` 1.0 :`G` 0.095177 :`A` 1.0))))
    (else
      (bind _returnvalue_3 (`GameplayStatics.CreateSaveGameObject` "/Game/BP_SaveSTP.BP_SaveSTP_C"))
      (set `self.UserSettings` _returnvalue_3)
      (goto _label))))

(fn `SaveUserSettings`
  (bind _returnvalue (`GameplayStatics.DoesSaveGameExist` (`self.UserSettingsSlot`)))
  (if (not _returnvalue)
    (bind _returnvalue_2 (`GameplayStatics.CreateSaveGameObject` "/Game/BP_SaveSTP.BP_SaveSTP_C"))
    (set `self.UserSettings` _returnvalue_2))
  (set `/Game/BP_SaveSTP.LatestSaveGame` (`self.CurrentSlot`) (`self.UserSettings`))
  (`GameplayStatics.SaveGameToSlot` (`self.UserSettings`) (`self.UserSettingsSlot`)))

(fn `ToggleMusic`
  (params (NewValue :type Boolean))
  (`GameplayStatics.SetSoundMixClassOverride` "/Game/Menu/SFX/SoundMix_Master.SoundMix_Master" "/Game/Menu/SFX/SoundClass_Music.SoundClass_Music" (`KismetMathLibrary.SelectFloat` (`.Music_2_57FCFFE141F8EA0FF3F29091468005C3` (break `/Game/Menu/S_AudioMix` (`/Game/BP_SaveSTP.AudioMixer` (`self.UserSettings`)))) 0.001 NewValue) 1.0 0.0) ; SFX
  (setmembers `/Game/Menu/S_AudioMix` :`StructRef` (`/Game/BP_SaveSTP.AudioMixer` (`self.UserSettings`)) :`Music Enabled` (`local.NewValue`)))

(fn `ToggleSound`
  (params (NewValue :type Boolean))
  (`GameplayStatics.SetSoundMixClassOverride` "/Game/Menu/SFX/SoundMix_Master.SoundMix_Master" "/Game/Menu/SFX/SoundClass_SFX.SoundClass_SFX" (`KismetMathLibrary.SelectFloat` (`.Effects_4_2E8E333C437F0AC6675871BC4511A3F6` (break `/Game/Menu/S_AudioMix` (`/Game/BP_SaveSTP.AudioMixer` (`self.UserSettings`)))) 0.001 NewValue) 1.0 0.0) ; SFX
  (setmembers `/Game/Menu/S_AudioMix` :`StructRef` (`/Game/BP_SaveSTP.AudioMixer` (`self.UserSettings`)) :`SFX Enabled` (`local.NewValue`)))

(fn `UpdateSoundMix`
  (params (NewVolume :type "Float (double-precision)"))
  (`GameplayStatics.SetSoundMixClassOverride` "/Game/Menu/SFX/SoundMix_Master.SoundMix_Master" "/Game/Menu/SFX/SoundClass_Master.SoundClass_Master" (`KismetMathLibrary.FMax` (`local.NewVolume`) 0.001) 1.0 0.0)
  (`GameplayStatics.PushSoundMixModifier` "/Game/Menu/SFX/SoundMix_Master.SoundMix_Master")
  (setmembers `/Game/Menu/S_AudioMix` :`StructRef` (`/Game/BP_SaveSTP.AudioMixer` (`self.UserSettings`)) :`Master` (`local.NewVolume`)))