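; Game mode for the working computer and Wi-Fi feature that picks a random password (MDP) when play begins.
; BeginPlay clears LongString, builds an array from three preset password variables, then calls GetRandomPassword.
; That function stores a random entry as MDP and its character count as MDPLIMIT, printing both to screen.
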(event `self.ReceiveBeginPlay`
  (set `self.Long string` "")
  (set `self.MDP_array` (`|MakeArray` (`self.MDP_1`) (`self.MDP_2`) (`self.MDP_3`)))
  (`self.Get Random Password`))

(fn `Get Random Password`
  (bind _mdp_array (`self.MDP_array`))
  (bind _output_get (set `self.MDP` (`|GetArrayItem` _mdp_array (`KismetMathLibrary.RandomIntegerInRange` 0 (`KismetArrayLibrary.Array_LastIndex` _mdp_array)))))
  (`KismetSystemLibrary.PrintString` _output_get true true (struct :`G` 0.399046 :`B` 1.0 :`A` 1.0) 10.0 "None")
  (bind _output_get_2 (set `self.MDP_LIMIT` (`KismetArrayLibrary.Array_Length` (`KismetStringLibrary.GetCharacterArrayFromString` _output_get))))
  (`KismetSystemLibrary.PrintString` (`KismetStringLibrary.Conv_IntToString` _output_get_2) true true (struct :`R` 1.0 :`G` 0.513763 :`A` 1.0) 10.0 "None"))

(fn `UserConstructionScript`)