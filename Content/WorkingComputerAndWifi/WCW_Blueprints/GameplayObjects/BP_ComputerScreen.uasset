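; BP_ComputerScreen is a computer monitor actor that hosts the WG_MainScreen widget and can link to a PC by cable.
; On BeginPlay it registers itself with the widget and turns on, toggling widget visibility and ticking, Wi-Fi list refresh and emissive material.
; Cable removal clears both ends when the screen owns the cable, otherwise delegates to the owning BP_ComputerCase.
; A helper plays sounds or media on separate audio components at the set volume.
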(event `self.ReceiveTick`
  (params (DeltaSeconds :type "Float (single-precision)")))

(event `self.ReceiveBeginPlay`
  ;[0.05098 0.05098 0.05098] Set this screen as the one owning the widget
  (bind _aswg_main_screen (cast `/Game/WorkingComputerAndWifi/WCW_Blueprints/Widgets/WG_MainScreen` (`WidgetComponent.GetWidget` (`self.MainScreenWidget`))))
  (set `/Game/WorkingComputerAndWifi/WCW_Blueprints/Widgets/WG_MainScreen.Owning Computer Screen` self _aswg_main_screen)
  (set `self.WG_MainScreen Ref` _aswg_main_screen)
  (`self.Turn On/Off Screen` true))

(fn `Destroy Cable`
  (bind _cablecomponent (`self.CableComponent`)
    (:`then`
      (bind _returnvalue (`ActorComponent.GetOwner` _cablecomponent))
      (if (== _returnvalue self)
        (bind _connected_pc (`self.Connected PC`)
          (:`then`
            (set `/Game/WorkingComputerAndWifi/WCW_Blueprints/GameplayObjects/BP_ComputerCase.Connected Screen` null _connected_pc)
            (set `/Game/WorkingComputerAndWifi/WCW_Blueprints/GameplayObjects/BP_ComputerCase.CableComponent` null _connected_pc))
          (:`else`
            _))
        (`ActorComponent.K2_DestroyComponent` _cablecomponent)
        (else
          (bind _asbp_computer_case (cast `/Game/WorkingComputerAndWifi/WCW_Blueprints/GameplayObjects/BP_ComputerCase` _returnvalue))
          (`/Game/WorkingComputerAndWifi/WCW_Blueprints/GameplayObjects/BP_ComputerCase.Destroy Cable` _asbp_computer_case)))
      (set `self.Connected PC` null)
      (set `self.CableComponent` null))
    (:`else`)))

(fn `Play Sound / Media`
  (params (`Sound (T) / Media (F)` :type Boolean) (`Sound / Media to play` :type "SoundBase Object Reference"))
  (bind _audio_mediaplayer (`self.Audio_MediaPlayer`))
  (bind _audio_sounds (`self.Audio_Sounds`))
  (if `Sound (T) / Media (F)`
    (set `AudioComponent.VolumeMultiplier` (`self.Volume`) _audio_sounds)
    (`AudioComponent.SetSound` _audio_sounds `Sound / Media to play`)
    (`AudioComponent.Play` _audio_sounds 0.0)
    (else
      (set `AudioComponent.VolumeMultiplier` (`self.Volume`) _audio_mediaplayer)
      (`AudioComponent.SetSound` _audio_mediaplayer `Sound / Media to play`)
      (`AudioComponent.Play` _audio_mediaplayer 0.0))))

(fn `Turn On/Off Screen`
  (params (`Turn On (t) / Off (f)` :type Boolean))
  (bind _mainscreenwidget (`self.MainScreenWidget`))
  (bind _mainscreenwidget_2 (`self.MainScreenWidget`))
  (bind _sm_computerscreen (`self.SM_ComputerScreen`))
  (if `Turn On (t) / Off (f)`
    (`ActorComponent.SetComponentTickEnabled` _mainscreenwidget true)
    (`SceneComponent.SetVisibility` _mainscreenwidget true false)
    (bind _wg_mainscreen_ref (`self.WG_MainScreen Ref`)
      (:`then`
        (`/Game/WorkingComputerAndWifi/WCW_Blueprints/Widgets/WG_MainScreen.Start/Stop updating Wifi List` _wg_mainscreen_ref true 10.0)
        (`MeshComponent.SetVectorParameterValueOnMaterials` _sm_computerscreen "EmissiveColor" (1.0 1.0 1.0))
        (`MeshComponent.SetScalarParameterValueOnMaterials` _sm_computerscreen "EmissiveStrength" 10.0)
        (`Widget.SetVisibility` (`/Game/WorkingComputerAndWifi/WCW_Blueprints/Widgets/WG_MainScreen.CanvasPanel_TurnOffPC` _wg_mainscreen_ref) "Collapsed"))
      (:`else`))
    (else
      (`ActorComponent.SetComponentTickEnabled` _mainscreenwidget_2 false)
      (`SceneComponent.SetVisibility` _mainscreenwidget_2 false false)
      (bind _wg_mainscreen_ref_2 (`self.WG_MainScreen Ref`)
        (:`then`
          (`/Game/WorkingComputerAndWifi/WCW_Blueprints/Widgets/WG_MainScreen.Start/Stop updating Wifi List` _wg_mainscreen_ref_2 false 0.0)
          (`MeshComponent.SetVectorParameterValueOnMaterials` (`self.SM_ComputerScreen`) "EmissiveColor" (0.0 0.0 0.0))
          (`MeshComponent.SetScalarParameterValueOnMaterials` _sm_computerscreen "EmissiveStrength" 0.0)
          (`Widget.SetVisibility` (`/Game/WorkingComputerAndWifi/WCW_Blueprints/Widgets/WG_MainScreen.CanvasPanel_TurnOffPC` _wg_mainscreen_ref_2) "Collapsed"))
        (:`else`)))))

(fn `UserConstructionScript`)