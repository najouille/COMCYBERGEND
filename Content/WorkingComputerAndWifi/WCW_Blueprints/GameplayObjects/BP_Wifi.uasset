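; Wi-Fi router actor that tracks which computers and security cameras are in range.
; A sphere's overlaps register it with computer cases and fill its reachable camera list; leaving disconnects a computer, updating its screen and stopping camera viewing.
; Switching swaps glow material parameters and sets the radius to zero or full, refreshing overlaps; game load reapplies this, delaying the radius.
; TurnOnOffWifi sets OnOff true in both branches, so it never stores off.
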(event `GameLoaded`
  (bind _sm_wifi (`self.SM_Wifi`))
  (bind _sm_wifi_2 (`self.SM_Wifi`))
  ;[0.03646 0.03646 0.03646] On load - We have a function for this (Turn On/Off Wifi) but on game load, we need it to be switched
  (if (`self.On/Off`)
    ;;[0.05098 0.05098 0.05098] Materials
    (`MeshComponent.SetVectorParameterValueOnMaterials` _sm_wifi_2 "On/Off Color" (0.0 0.45 0.0)) ; Green Color
    (`MeshComponent.SetScalarParameterValueOnMaterials` _sm_wifi_2 "On/Off_Strength" 20.0)
    (`KismetSystemLibrary.Delay` 2.0)
    (`SphereComponent.SetSphereRadius` (`self.Wifi Radius Component`) (`self.Wifi Radius`) true)
    (else
      (`MeshComponent.SetVectorParameterValueOnMaterials` _sm_wifi "On/Off Color" (0.0 0.0 0.0)) ; Green Color
      (`MeshComponent.SetScalarParameterValueOnMaterials` _sm_wifi "On/Off_Strength" 0.0)
      (`KismetSystemLibrary.Delay` 2.0)
      (`SphereComponent.SetSphereRadius` (`self.Wifi Radius Component`) 0.0 true))))

(event `self.Wifi Radius Component.OnComponentBeginOverlap`
  (params (OverlappedComponent :type "PrimitiveComponent Object Reference") (OtherActor :type "Actor Object Reference") (OtherComp :type "PrimitiveComponent Object Reference") (OtherBodyIndex :type Integer) (bFromSweep :type Boolean) (SweepResult :type "HitResult Structure (by ref)"))
  (bind _reachable_security_cameras (`self.Reachable Security Cameras`))
  ;[0.05098 0.05098 0.05098] Handling Wi-FI reachable radius for Computers and Security Cameras
  ;;[1 1 1] Begin Reaching
  (`|ExecutionSequence`
    (:`then_0`
      (bind _asbp_computer_case (cast `/Game/WorkingComputerAndWifi/WCW_Blueprints/GameplayObjects/BP_ComputerCase` OtherActor))
      (bind _available_wifi_list (`/Game/WorkingComputerAndWifi/WCW_Blueprints/GameplayObjects/BP_ComputerCase.Available Wifi List` _asbp_computer_case))
      (if (not (`KismetArrayLibrary.Array_Contains` _available_wifi_list self))
        (`KismetArrayLibrary.Array_Add` _available_wifi_list self)))
    (:`then_1`
      (bind _asbp_security_camera (cast `/Game/WorkingComputerAndWifi/WCW_Blueprints/GameplayObjects/BP_SecurityCamera` OtherActor))
      (if (not (`KismetArrayLibrary.Array_Contains` _reachable_security_cameras _asbp_security_camera))
        (`KismetArrayLibrary.Array_Add` _reachable_security_cameras _asbp_security_camera)))))

(event `self.Wifi Radius Component.OnComponentEndOverlap`
  (params (OverlappedComponent :type "PrimitiveComponent Object Reference") (OtherActor :type "Actor Object Reference") (OtherComp :type "PrimitiveComponent Object Reference") (OtherBodyIndex :type Integer))
  (bind _reachable_security_cameras (`self.Reachable Security Cameras`))
  ;[0.05098 0.05098 0.05098] Handling Wi-FI reachable radius for Computers and Security Cameras
  ;;[1 1 1] Stop reaching
  (`|ExecutionSequence`
    (:`then_0`
      (bind _asbp_computer_case (cast `/Game/WorkingComputerAndWifi/WCW_Blueprints/GameplayObjects/BP_ComputerCase` OtherActor))
      (bind _available_wifi_list (`/Game/WorkingComputerAndWifi/WCW_Blueprints/GameplayObjects/BP_ComputerCase.Available Wifi List` _asbp_computer_case))
      (if (`KismetArrayLibrary.Array_Contains` _available_wifi_list self)
        (`KismetArrayLibrary.Array_RemoveItem` _available_wifi_list self)
        (if (== (`/Game/WorkingComputerAndWifi/WCW_Blueprints/GameplayObjects/BP_ComputerCase.Connected Wifi` _asbp_computer_case) self)
          (`|ExecutionSequence`
            (:`then_0`
              (bind _connected_screen (`/Game/WorkingComputerAndWifi/WCW_Blueprints/GameplayObjects/BP_ComputerCase.Connected Screen` _asbp_computer_case)
                (:`then`
                  (bind _wg_mainscreen_ref (`/Game/WorkingComputerAndWifi/WCW_Blueprints/GameplayObjects/BP_ComputerScreen.WG_MainScreen Ref` _connected_screen))
                  (`/Game/WorkingComputerAndWifi/WCW_Blueprints/Widgets/WG_MainScreen.Set Wifi Icon (Connected/Disconnected)` _wg_mainscreen_ref false)
                  (`/Game/WorkingComputerAndWifi/WCW_Blueprints/Widgets/WG_MainScreen.Set Available Wifi List` _wg_mainscreen_ref)
                  (bind _security (`/Game/WorkingComputerAndWifi/WCW_Blueprints/Widgets/WG_MainScreen.Security` _wg_mainscreen_ref))
                  (`/Game/WorkingComputerAndWifi/WCW_Blueprints/Widgets/App5_Security/Security.Current Viewed Camera` _security
                    (:`then`
                      (`/Game/WorkingComputerAndWifi/WCW_Blueprints/Widgets/App5_Security/Security.Stop watching camera` _security))
                    (:`else`)))
                (:`else`)))
            (:`then_1`
              (set `/Game/WorkingComputerAndWifi/WCW_Blueprints/GameplayObjects/BP_ComputerCase.Connected Wifi` null _asbp_computer_case))))))
    (:`then_1`
      (bind _asbp_security_camera (cast `/Game/WorkingComputerAndWifi/WCW_Blueprints/GameplayObjects/BP_SecurityCamera` OtherActor))
      (`|ExecutionSequence`
        (:`then_0`
          (if (`KismetArrayLibrary.Array_Contains` _reachable_security_cameras _asbp_security_camera)
            (`KismetArrayLibrary.Array_RemoveItem` _reachable_security_cameras _asbp_security_camera)))))))

(fn `Turn On/Off Wifi`
  (bind _sm_wifi (`self.SM_Wifi`))
  (bind _sm_wifi_2 (`self.SM_Wifi`))
  (if (`self.On/Off`)
    ;[0.05098 0.05098 0.05098] Materials
    (`MeshComponent.SetVectorParameterValueOnMaterials` _sm_wifi "On/Off Color" (0.0 0.0 0.0)) ; Green Color
    (`MeshComponent.SetScalarParameterValueOnMaterials` _sm_wifi "On/Off_Strength" 0.0)
    (`SphereComponent.SetSphereRadius` (`self.Wifi Radius Component`) 0.0 true)
    (set `self.On/Off` true)
    (else
      (`MeshComponent.SetVectorParameterValueOnMaterials` _sm_wifi_2 "On/Off Color" (0.0 0.45 0.0)) ; Green Color
      (`MeshComponent.SetScalarParameterValueOnMaterials` _sm_wifi_2 "On/Off_Strength" 20.0)
      (`SphereComponent.SetSphereRadius` (`self.Wifi Radius Component`) (`self.Wifi Radius`) true)
      (set `self.On/Off` true))))

(fn `UserConstructionScript`)