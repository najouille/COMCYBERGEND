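; BP_Keyboard is a keyboard actor that links wirelessly by proximity to a BP_ComputerCase and lights up while connected.
; After a short BeginPlay delay it sets the connection sphere's radius, forcing overlaps to register even if the keyboard loads before the PC.
; Overlap begin and end drive ConnectDisconnectPC, which keeps a single two-way reference with the PC.
; That function also toggles the keyboard material and copies the PC's RGB color and strength when enabled.
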(event `self.ReceiveBeginPlay`
  ;[0.05098 0.05098 0.05098] A little delay to update overlaps when the game starts. It can happen that keyboard loads faster than a computer and therefore would end up no connecting to PC.
  ;
  ; Sphere radius should be kept at "0". Set the "Sphere Radius Variable" to your requested number and it will be set automatically at the beginning. It is all just so the overlaps are updated as the game begins.
  (`KismetSystemLibrary.Delay` 2.0)
  (`SphereComponent.SetSphereRadius` (`self.Connection radius`) (`self.Sphere Radius`) true))

(event `self.Connection radius.OnComponentBeginOverlap`
  (params (OverlappedComponent :type "PrimitiveComponent Object Reference") (OtherActor :type "Actor Object Reference") (OtherComp :type "PrimitiveComponent Object Reference") (OtherBodyIndex :type Integer) (bFromSweep :type Boolean) (SweepResult :type "HitResult Structure (by ref)"))
  ;[0.05098 0.05098 0.05098] Begin Overlap
  (bind _asbp_computer_case (cast `/Game/WorkingComputerAndWifi/WCW_Blueprints/GameplayObjects/BP_ComputerCase` OtherActor))
  (`self.Connect / Disconnect PC` true _asbp_computer_case))

(event `self.Connection radius.OnComponentEndOverlap`
  (params (OverlappedComponent :type "PrimitiveComponent Object Reference") (OtherActor :type "Actor Object Reference") (OtherComp :type "PrimitiveComponent Object Reference") (OtherBodyIndex :type Integer))
  (bind _connected_pc (`self.Connected PC`))
  ;[0.05098 0.05098 0.05098] Begin Overlap
  (if (== OtherActor _connected_pc)
    (`self.Connect / Disconnect PC` false _connected_pc)))

(fn `Connect / Disconnect PC`
  (params (`Connect (T) / Disconnect (F)` :type Boolean) (`PC to Connect / Disconnect` :type "/Game/WorkingComputerAndWifi/WCW_Blueprints/GameplayObjects/BP_ComputerCase Object Reference"))
  (bind _keyboard (`self.Keyboard`))
  (if `Connect (T) / Disconnect (F)`
    (`self.Connected PC`
      (:`then`)
      (:`else`
        (set `/Game/WorkingComputerAndWifi/WCW_Blueprints/GameplayObjects/BP_ComputerCase.Connected Keyboard` self `PC to Connect / Disconnect`)
        (bind _output_get (set `self.Connected PC` `PC to Connect / Disconnect`))
        (`MeshComponent.SetScalarParameterValueOnMaterials` _keyboard "On/Off" 1.0)
        (if (`/Game/WorkingComputerAndWifi/WCW_Blueprints/GameplayObjects/BP_ComputerCase.RGB on?` _output_get)
          (`MeshComponent.SetVectorParameterValueOnMaterials` _keyboard "RGB_Color" (`/Game/WorkingComputerAndWifi/WCW_Blueprints/GameplayObjects/BP_ComputerCase.RGB values` _output_get))
          (`MeshComponent.SetScalarParameterValueOnMaterials` _keyboard "RGB_Strength" (`/Game/WorkingComputerAndWifi/WCW_Blueprints/GameplayObjects/BP_ComputerCase.RGB strength` _output_get)))))
    (else
      (bind _connected_pc (`self.Connected PC`)
        (:`then`
          (set `/Game/WorkingComputerAndWifi/WCW_Blueprints/GameplayObjects/BP_ComputerCase.Connected Keyboard` null _connected_pc)
          (set `self.Connected PC` null)
          (`MeshComponent.SetScalarParameterValueOnMaterials` (`self.Keyboard`) "On/Off" 0.0)
          (`MeshComponent.SetVectorParameterValueOnMaterials` _keyboard "RGB_Color" (0.0208 0.0208 0.0208))
          (`MeshComponent.SetScalarParameterValueOnMaterials` _keyboard "RGB_Strength" 0.0))
        (:`else`)))))

(fn `UserConstructionScript`)