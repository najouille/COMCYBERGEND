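; Computer case actor that players can power on and off and link by cable to a BP_ComputerScreen.
; TurnOnOffPC toggles the connected screen and the case's glow material parameters; only RGB models also get color, button sound and delayed fan audio through one shared audio component.
; DestroyCable clears the link, delegating destruction to the screen if it owns the cable.
; Debug prints for Wifi, power and screen are unwired.
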(event `self.ReceiveTick`
  (params (DeltaSeconds :type "Float (single-precision)")))

(event `Start Fan Sound`
  ;[0.05098 0.05098 0.05098] Start fan sounds
  (`KismetSystemLibrary.Delay` 1.5)
  (`self.Play Sound` "/Game/WorkingComputerAndWifi/WCW_Blueprints/Sounds/ComputerSounds/Computer_Fans.Computer_Fans" 1.0))

(event `Stop Fan Sound`
  ;[0.05098 0.05098 0.05098] Stop fan sounds
  (`KismetSystemLibrary.Delay` 1.5)
  (`AudioComponent.Stop` (`self.Audio`)))

(fn `Destroy Cable`
  (bind _cablecomponent (`self.CableComponent`)
    (:`then`
      (bind _returnvalue (`ActorComponent.GetOwner` _cablecomponent))
      (if (== _returnvalue self)
        (bind _connected_screen (`self.Connected Screen`)
          (:`then`
            (set `/Game/WorkingComputerAndWifi/WCW_Blueprints/GameplayObjects/BP_ComputerScreen.Connected PC` null _connected_screen)
            (set `/Game/WorkingComputerAndWifi/WCW_Blueprints/GameplayObjects/BP_ComputerScreen.CableComponent` null _connected_screen))
          (:`else`
            _))
        (`ActorComponent.K2_DestroyComponent` _cablecomponent)
        (else
          (bind _asbp_computer_screen (cast `/Game/WorkingComputerAndWifi/WCW_Blueprints/GameplayObjects/BP_ComputerScreen` _returnvalue))
          (`/Game/WorkingComputerAndWifi/WCW_Blueprints/GameplayObjects/BP_ComputerScreen.Destroy Cable` _asbp_computer_screen)))
      (set `self.Connected Screen` null)
      (set `self.CableComponent` null))
    (:`else`)))

(fn `Turn On/Off PC`
  (bind _sm_computercase (`self.SM_ComputerCase`))
  (bind _sm_computercase_2 (`self.SM_ComputerCase`))
  (bind (_rgb_values_x _rgb_values_y _rgb_values_z) (`KismetMathLibrary.BreakVector` (`self.RGB values`)))
  (if (`self.On/Off`)
    (bind _connected_screen (`self.Connected Screen`)
      (:`then`
        ;[0.05098 0.05098 0.05098] Turn On Screen (only when connected)
        (`/Game/WorkingComputerAndWifi/WCW_Blueprints/GameplayObjects/BP_ComputerScreen.Turn On/Off Screen` _connected_screen false))
      (:`else`
        _))
    ;[0.05098 0.05098 0.05098] Do always (Computer Only stuff)
    (`MeshComponent.SetScalarParameterValueOnMaterials` (`self.SM_ComputerCase`) "On/Off_Strength" 0.0)
    (set `self.On/Off` false)
    ;[0.05098 0.05098 0.05098] Do only on PC´s with RGB
    (if (`self.Has RGB?`)
      (`MeshComponent.SetScalarParameterValueOnMaterials` _sm_computercase_2 "RGB_Strength" 0.0)
      (`MeshComponent.SetVectorParameterValueOnMaterials` _sm_computercase_2 "RGB_Color" (0.0 0.0 0.0))
      ;[0.05098 0.05098 0.05098] Sounds
      (`self.Play Sound` "/Game/WorkingComputerAndWifi/WCW_Blueprints/Sounds/ComputerSounds/Button.Button" 1.0)
      (`self.Stop Fan Sound`))
    (else
      (bind _connected_screen_2 (`self.Connected Screen`)
        (:`then`
          (`/Game/WorkingComputerAndWifi/WCW_Blueprints/GameplayObjects/BP_ComputerScreen.Turn On/Off Screen` _connected_screen_2 true))
        (:`else`
          _))
      (`MeshComponent.SetScalarParameterValueOnMaterials` (`self.SM_ComputerCase`) "On/Off_Strength" 50.0)
      (set `self.On/Off` true)
      (if (`self.Has RGB?`)
        (`MeshComponent.SetScalarParameterValueOnMaterials` _sm_computercase "RGB_Strength" (`self.RGB strength`))
        (`MeshComponent.SetVectorParameterValueOnMaterials` _sm_computercase "RGB_Color" (`KismetMathLibrary.MakeVector` _rgb_values_x _rgb_values_y _rgb_values_z))
        (`self.Play Sound` "/Game/WorkingComputerAndWifi/WCW_Blueprints/Sounds/ComputerSounds/Button.Button" 1.0)
        (`self.Start Fan Sound`)))))

(fn `UserConstructionScript`)