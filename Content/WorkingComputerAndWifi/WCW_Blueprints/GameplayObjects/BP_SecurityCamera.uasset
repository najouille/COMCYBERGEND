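; BP_SecurityCamera is a switchable security camera that viewers watch on in-game computers, identified by a displayed serial number, randomly generated after BeginPlay if empty.
; It creates a render target on demand for its SceneCapture, captured manually on a looping timer that starts and stops by function call, with a debug warning each capture.
; Toggling updates a material parameter and plays a sound; switching off also releases the target and stops all current viewers watching.
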(event `self.ReceiveBeginPlay`
  (`KismetSystemLibrary.Delay` 2.0)
  (`self.Generate Serial Number`))

(fn `Create RenderTarget`
  (`SceneCaptureComponent2D.TextureTarget` (`self.SceneCapture`)
    (:`then`)
    (:`else`
      (bind _returnvalue (`KismetRenderingLibrary.CreateRenderTarget2D` 1920 1080))
      (bind _output_get (set `self.Render Target` _returnvalue))
      (set `SceneCaptureComponent2D.TextureTarget` _output_get (`self.SceneCapture`)))))

(fn `Destroy RenderTarget`
  (`SceneCaptureComponent2D.TextureTarget` (`self.SceneCapture`)
    (:`then`
      (set `self.Render Target` null)
      (set `SceneCaptureComponent2D.TextureTarget` null (`self.SceneCapture`))
      (bind (_arrayindex _arrayelement) (`/Engine/EditorBlueprintResources/StandardMacros.ReverseForEachLoop` (`self.Current Viewers`))
        (:`LoopBody`
          (`/Game/WorkingComputerAndWifi/WCW_Blueprints/Widgets/App5_Security/Security.Stop watching camera` (`/Game/WorkingComputerAndWifi/WCW_Blueprints/Widgets/WG_MainScreen.Security` (`/Game/WorkingComputerAndWifi/WCW_Blueprints/GameplayObjects/BP_ComputerScreen.WG_MainScreen Ref` _arrayelement))))))
    (:`else`)))

(fn `Generate Serial Number`
  (locals (Alphabet :type "Array of Text") (Numbers :type "Array of Text"))
  ;[0.05098 0.05098 0.05098] Generate random Serial Number
  (if (`KismetTextLibrary.TextIsEmpty` (`self.Serial Number`))
    (for _ (range 4)
      (set `self.Serial Number` (`KismetTextLibrary.Conv_StringToText` (`KismetStringLibrary.Concat_StrStr` (`KismetTextLibrary.Conv_TextToString` (`self.Serial Number`)) (`KismetTextLibrary.Conv_TextToString` (`KismetArrayLibrary.Array_Random` (`local.Alphabet`)))))))
    (for _ (range 3)
      (set `self.Serial Number` (`KismetTextLibrary.Conv_StringToText` (`KismetStringLibrary.Concat_StrStr` (`KismetTextLibrary.Conv_TextToString` (`self.Serial Number`)) (`KismetTextLibrary.Conv_TextToString` (`KismetArrayLibrary.Array_Random` (`local.Numbers`)))))))
    (for _ (range 3)
      (set `self.Serial Number` (`KismetTextLibrary.Conv_StringToText` (`KismetStringLibrary.Concat_StrStr` (`KismetTextLibrary.Conv_TextToString` (`self.Serial Number`)) (`KismetTextLibrary.Conv_TextToString` (`KismetArrayLibrary.Array_Random` (`local.Alphabet`))))))
      (`TextRenderComponent.K2_SetText` (`self.SerialNumber`) (`self.Serial Number`) :!label _label))
    (else
      (goto _label))))

(fn `Start Capturing Image`
  (`SceneCaptureComponent2D.CaptureScene` (`self.SceneCapture`))
  (`KismetSystemLibrary.K2_SetTimer` null "Start Capturing Image" 0.05 true)
  ;[1 0.3417 0] Debug
  (`KismetSystemLibrary.PrintString` (`KismetStringLibrary.Concat_StrStr` (`KismetSystemLibrary.GetDisplayName` self) " is capturing image! This event should not be running if you are not watching the camera on any computer. If it is, please report it to me ASAP (performance issue)") true true (struct :`R` 1.0 :`G` 0.057555 :`A` 1.0) 0.05))

(fn `Stop Capturing Image`
  (`KismetSystemLibrary.K2_ClearTimer` null "Start Capturing Image"))

(fn `Turn On/Off Camera`
  (if (`self.On/Off`)
    (`MeshComponent.SetScalarParameterValueOnMaterials` (`self.SecurityCamera`) "On/Off" 0.0)
    (set `self.On/Off` false)
    (`self.Destroy RenderTarget`)
    (`self.Play Sound` "/Game/WorkingComputerAndWifi/WCW_Blueprints/Sounds/ComputerSounds/Switch_Off.Switch_Off" 1.0)
    (else
      (`MeshComponent.SetScalarParameterValueOnMaterials` (`self.SecurityCamera`) "On/Off" 1.0)
      (set `self.On/Off` true)
      (`self.Play Sound` "/Game/WorkingComputerAndWifi/WCW_Blueprints/Sounds/ComputerSounds/Switch_On.Switch_On" 1.0))))

(fn `UserConstructionScript`)