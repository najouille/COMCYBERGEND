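; Game state for the computer and Wi-Fi game that saves world progress and calls LoadGame for Slot1 on BeginPlay.
; SaveGame writes email databases, player money and settings, Wi-Fi, notes, monitor links and security cameras into a Simple_SaveGame, gathering actors by class.
; LoadGame only loads and casts the save.
; Its restore logic, including rebuilding monitor cables, is disconnected and never runs.
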(event `self.ReceiveBeginPlay`
  (bind _asbp_wcw_player_state (cast `/Game/WorkingComputerAndWifi/WCW_Blueprints/BP_WCW_PlayerState` (`GameplayStatics.GetPlayerState` 0)))
  (`self.LoadGame` "Slot1" _asbp_wcw_player_state))

(fn `LoadGame`
  (params (SlotName :type String) (`Player State` :type "/Game/WorkingComputerAndWifi/WCW_Blueprints/BP_WCW_PlayerState Object Reference"))
  (bind _returnvalue (`GameplayStatics.DoesSaveGameExist` SlotName))
  (if _returnvalue
    (bind _returnvalue_2 (`GameplayStatics.LoadGameFromSlot` SlotName))
    (bind _assimple_save_game (cast `/Game/WorkingComputerAndWifi/WCW_Blueprints/Game_Save/Simple_SaveGame` _returnvalue_2))))

(fn `SaveGame`
  (params (SlotName :type String))
  (bind _returnvalue (`GameplayStatics.DoesSaveGameExist` SlotName))
  (if _returnvalue
    (bind _returnvalue_2 (`GameplayStatics.LoadGameFromSlot` SlotName))
    (set `self.Save Reference` _returnvalue_2)
    (else
      (bind _returnvalue_3 (`GameplayStatics.CreateSaveGameObject` "/Game/WorkingComputerAndWifi/WCW_Blueprints/Game_Save/Simple_SaveGame.Simple_SaveGame_C"))
      (set `self.Save Reference` _returnvalue_3)))
  (bind _assimple_save_game (cast `/Game/WorkingComputerAndWifi/WCW_Blueprints/Game_Save/Simple_SaveGame` (`self.Save Reference`)))
  (`|ExecutionSequence`
    (:`then_0`
      ;[0.03646 0.03646 0.03646] GameState - Database
      (set `/Game/WorkingComputerAndWifi/WCW_Blueprints/Game_Save/Simple_SaveGame.Database of E-Mail Messages` (`self.Database - E-Mail Messages`) _assimple_save_game)
      (set `/Game/WorkingComputerAndWifi/WCW_Blueprints/Game_Save/Simple_SaveGame.Database of Registered E-Mails` (`self.Database - Registered E-Mails`) _assimple_save_game))
    (:`then_1`
      ;[0.03646 0.03646 0.03646] PlayerState
      (bind _asbp_wcw_player_state (cast `/Game/WorkingComputerAndWifi/WCW_Blueprints/BP_WCW_PlayerState` (`GameplayStatics.GetPlayerState` 0)))
      (set `/Game/WorkingComputerAndWifi/WCW_Blueprints/Game_Save/Simple_SaveGame.PlayerMoney` (`/Game/WorkingComputerAndWifi/WCW_Blueprints/BP_WCW_PlayerState.Player Money` _asbp_wcw_player_state) _assimple_save_game)
      (set `/Game/WorkingComputerAndWifi/WCW_Blueprints/Game_Save/Simple_SaveGame.PlayerSettings` (`/Game/WorkingComputerAndWifi/WCW_Blueprints/BP_WCW_PlayerState.Player Settings` _asbp_wcw_player_state) _assimple_save_game))
    (:`then_2`
      (bind _wi_fi_variables (`/Game/WorkingComputerAndWifi/WCW_Blueprints/Game_Save/Simple_SaveGame.Wi-Fi variables` _assimple_save_game))
      ;[0.03646 0.03646 0.03646] Wi-Fi
      (`KismetArrayLibrary.Array_Clear` _wi_fi_variables)
      (bind _outactors (`GameplayStatics.GetAllActorsOfClass` "/Game/WorkingComputerAndWifi/WCW_Blueprints/GameplayObjects/BP_Wifi.BP_Wifi_C"))
      (for _array_element _outactors
        (`KismetArrayLibrary.Array_Add` _wi_fi_variables (make `/Game/WorkingComputerAndWifi/WCW_Blueprints/Enums_And_Structs/S_Save_Wi-Fi` _array_element (`/Game/WorkingComputerAndWifi/WCW_Blueprints/GameplayObjects/BP_Wifi.Wi-Fi Name` _array_element) (`/Game/WorkingComputerAndWifi/WCW_Blueprints/GameplayObjects/BP_Wifi.Wi-Fi Password` _array_element) (`/Game/WorkingComputerAndWifi/WCW_Blueprints/GameplayObjects/BP_Wifi.On/Off` _array_element)))))
    (:`then_3`
      (bind _computer_apps (`/Game/WorkingComputerAndWifi/WCW_Blueprints/Game_Save/Simple_SaveGame.Computer Apps` _assimple_save_game))
      ;[0.03646 0.03646 0.03646] Computer Apps
      (`KismetArrayLibrary.Array_Clear` _computer_apps)
      (bind _outactors_2 (`GameplayStatics.GetAllActorsOfClass` "/Game/WorkingComputerAndWifi/WCW_Blueprints/GameplayObjects/BP_ComputerScreen.BP_ComputerScreen_C"))
      (for _array_element_2 _outactors_2
        (`KismetArrayLibrary.Array_Add` _computer_apps (make `/Game/WorkingComputerAndWifi/WCW_Blueprints/Enums_And_Structs/S_Save_ComputerApps` _array_element_2 (`MultiLineEditableTextBox.GetText` (`/Game/WorkingComputerAndWifi/WCW_Blueprints/Widgets/App7_Notes/Notes.TextBlock` (`/Game/WorkingComputerAndWifi/WCW_Blueprints/Widgets/WG_MainScreen.Notes` (`/Game/WorkingComputerAndWifi/WCW_Blueprints/GameplayObjects/BP_ComputerScreen.WG_MainScreen Ref` _array_element_2))))))))
    (:`then_4`
      (bind _computer_connection_to_monitor (`/Game/WorkingComputerAndWifi/WCW_Blueprints/Game_Save/Simple_SaveGame.Computer Connection to Monitor` _assimple_save_game))
      ;[0.03646 0.03646 0.03646] Computer -> Screen Connections
      (`KismetArrayLibrary.Array_Clear` _computer_connection_to_monitor)
      (bind _outactors_3 (`GameplayStatics.GetAllActorsOfClass` "/Game/WorkingComputerAndWifi/WCW_Blueprints/GameplayObjects/BP_ComputerCase.BP_ComputerCase_C"))
      (for _array_element_3 _outactors_3
        (bind _connected_screen (`/Game/WorkingComputerAndWifi/WCW_Blueprints/GameplayObjects/BP_ComputerCase.Connected Screen` _array_element_3)
          (:`then`
            (`KismetArrayLibrary.Array_Add` _computer_connection_to_monitor (make `/Game/WorkingComputerAndWifi/WCW_Blueprints/Enums_And_Structs/S_Save_ComputerConnection` _array_element_3 _connected_screen)))
          (:`else`))))
    (:`then_5`
      (bind _security_cameras_status (`/Game/WorkingComputerAndWifi/WCW_Blueprints/Game_Save/Simple_SaveGame.Security Cameras Status` _assimple_save_game))
      ;[0.03646 0.03646 0.03646] Security Cameras
      (`KismetArrayLibrary.Array_Clear` _security_cameras_status)
      (bind _outactors_4 (`GameplayStatics.GetAllActorsOfClass` "/Game/WorkingComputerAndWifi/WCW_Blueprints/GameplayObjects/BP_SecurityCamera.BP_SecurityCamera_C"))
      (for _array_element_4 _outactors_4
        (`KismetArrayLibrary.Array_Add` _security_cameras_status (make `/Game/WorkingComputerAndWifi/WCW_Blueprints/Enums_And_Structs/S_Save_CameraState` _array_element_4 (`/Game/WorkingComputerAndWifi/WCW_Blueprints/GameplayObjects/BP_SecurityCamera.Serial Number` _array_element_4) (`/Game/WorkingComputerAndWifi/WCW_Blueprints/GameplayObjects/BP_SecurityCamera.Camera Name` _array_element_4) (`/Game/WorkingComputerAndWifi/WCW_Blueprints/GameplayObjects/BP_SecurityCamera.On/Off` _array_element_4) (`/Game/WorkingComputerAndWifi/WCW_Blueprints/GameplayObjects/BP_SecurityCamera.Trusted Network` _array_element_4)))))
    (:`then_6`
      ;[0 1 0.004799] Game Save
      (bind _returnvalue_4 (`GameplayStatics.SaveGameToSlot` (`self.Save Reference`) SlotName))
      (if _returnvalue_4
        (`KismetSystemLibrary.PrintString` "Game Saved!")
        (else
          (`KismetSystemLibrary.PrintString` "Failed to Save!"))))))

(fn `UserConstructionScript`)