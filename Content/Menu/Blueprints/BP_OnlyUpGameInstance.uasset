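; Game instance for the Only Up game that holds user settings and applies audio volumes and toggles.
; Settings load lazily from a BP_SaveSTP save slot, or a new object if none exists, then initialize the audio mix.
; Volume and toggle functions override SoundMix_Master classes and update the settings struct, using a 0.001 floor instead of zero to keep sounds alive.
; SaveUserSettings separately writes the settings and current slot to disk.
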(fn `GetUserSettings`
  (returns (UserSettings :type "Object Object Reference"))
  (bind _usersettings (`self.UserSettings`)
    (:`then`
      (return _usersettings))
    (:`else`
      (`self.LoadUserSettings`)
      (return (`self.UserSettings`)))))

(fn `InitAudioMixSettings`
  (bind (_master _music _effects _musicenabled _sfxenabled) (break `/Game/Menu/S_AudioMix` (`/Game/BP_SaveSTP.AudioMixer` (`self.UserSettings`))))
  (bind (_master_2 _music_2 _effects_2 _musicenabled_2) (break `/Game/Menu/S_AudioMix` (`/Game/BP_SaveSTP.AudioMixer` (`self.UserSettings`))))
  (`|ExecutionSequence`
    (:`then_0`
      (`GameplayStatics.SetSoundMixClassOverride` "/Game/Menu/SFX/SoundMix_Master.SoundMix_Master" "/Game/Menu/SFX/SoundClass_Master.SoundClass_Master" (`KismetMathLibrary.SelectFloat` (`.Master_6_5C15BA8347FB14327EF9EE9156A9D623` (break `/Game/Menu/S_AudioMix` (`/Game/BP_SaveSTP.AudioMixer` (`self.UserSettings`)))) 0.001) 1.0 0.0))
    (:`then_1`
      (`GameplayStatics.SetSoundMixClassOverride` "/Game/Menu/SFX/SoundMix_Master.SoundMix_Master" "/Game/Menu/SFX/SoundClass_Music.SoundClass_Music" (`KismetMathLibrary.SelectFloat` _music_2 0.001 _musicenabled_2) 1.0 0.0))
    (:`then_2`
      (`GameplayStatics.SetSoundMixClassOverride` "/Game/Menu/SFX/SoundMix_Master.SoundMix_Master" "/Game/Menu/SFX/SoundClass_SFX.SoundClass_SFX" (`KismetMathLibrary.SelectFloat` _effects 0.001 _sfxenabled) 1.0 0.0))))

(fn `InitUserSettings`
  (`self.InitAudioMixSettings`))

(fn `LoadUserSettings`
  (bind _returnvalue (`GameplayStatics.DoesSaveGameExist` (`self.UserSettingsSlot`)))
  (if _returnvalue
    (bind _returnvalue_2 (`GameplayStatics.LoadGameFromSlot` (`self.UserSettingsSlot`)))
    (bind _asbp_save_stp (cast `/Game/BP_SaveSTP` _returnvalue_2))
    (set `self.UserSettings` _asbp_save_stp)
    (else
      (bind _returnvalue_3 (`GameplayStatics.CreateSaveGameObject` "/Game/BP_SaveSTP.BP_SaveSTP_C"))
      (set `self.UserSettings` _returnvalue_3)))
  (`self.InitUserSettings`)
  (return))

(fn `SaveUserSettings`
  (bind _returnvalue (`GameplayStatics.DoesSaveGameExist` (`self.UserSettingsSlot`)))
  (if (not _returnvalue)
    (bind _returnvalue_2 (`GameplayStatics.CreateSaveGameObject` "/Game/BP_SaveSTP.BP_SaveSTP_C"))
    (set `self.UserSettings` _returnvalue_2))
  (set `/Game/BP_SaveSTP.LatestSaveGame` (`self.CurrentSlot`) (`self.UserSettings`))
  (`GameplayStatics.SaveGameToSlot` (`self.UserSettings`) (`self.UserSettingsSlot`)))

(fn `ToggleMusic`
  (params (NewValue :type Boolean))
  (`GameplayStatics.SetSoundMixClassOverride` "/Game/Menu/SFX/SoundMix_Master.SoundMix_Master" "/Game/Menu/SFX/SoundClass_Music.SoundClass_Music" (`KismetMathLibrary.SelectFloat` (`.Music_2_57FCFFE141F8EA0FF3F29091468005C3` (break `/Game/Menu/S_AudioMix` (`/Game/BP_SaveSTP.AudioMixer` (`self.UserSettings`)))) 0.001 NewValue) 1.0 0.0) ; SFX
  (setmembers `/Game/Menu/S_AudioMix` :`StructRef` (`/Game/BP_SaveSTP.AudioMixer` (`self.UserSettings`)) :`Music Enabled` (`local.NewValue`)))

(fn `ToggleSound`
  (params (NewValue :type Boolean))
  (`GameplayStatics.SetSoundMixClassOverride` "/Game/Menu/SFX/SoundMix_Master.SoundMix_Master" "/Game/Menu/SFX/SoundClass_SFX.SoundClass_SFX" (`KismetMathLibrary.SelectFloat` (`.Effects_4_2E8E333C437F0AC6675871BC4511A3F6` (break `/Game/Menu/S_AudioMix` (`/Game/BP_SaveSTP.AudioMixer` (`self.UserSettings`)))) 0.001 NewValue) 1.0 0.0) ; SFX
  (setmembers `/Game/Menu/S_AudioMix` :`StructRef` (`/Game/BP_SaveSTP.AudioMixer` (`self.UserSettings`)) :`SFX Enabled` (`local.NewValue`)))

(fn `UpdateSoundMix`
  (params (InSoundClass :type "/Game/Menu/SFX/E_SoundClasses Enum" :default "NewEnumerator0") (NewVolume :type "Float (double-precision)"))
  (`GameplayStatics.SetSoundMixClassOverride` "/Game/Menu/SFX/SoundMix_Master.SoundMix_Master" (select `byte` InSoundClass :`0` "/Game/Menu/SFX/SoundClass_Master.SoundClass_Master" :`1` "/Game/Menu/SFX/SoundClass_Music.SoundClass_Music" :`2` "/Game/Menu/SFX/SoundClass_SFX.SoundClass_SFX" :!type "SoundClass Object Reference") (`KismetMathLibrary.FMax` (`local.NewVolume`) 0.001) 1.0 0.0)
  (switch `/Game/Menu/SFX/E_SoundClasses` (`local.InSoundClass`)
    (:`NewEnumerator0`
      (setmembers `/Game/Menu/S_AudioMix` :`StructRef` (`/Game/BP_SaveSTP.AudioMixer` (`self.UserSettings`)) :`Master` (`local.NewVolume`)))
    (:`NewEnumerator1`
      (setmembers `/Game/Menu/S_AudioMix` :`StructRef` (`/Game/BP_SaveSTP.AudioMixer` (`self.UserSettings`)) :`Music` (`local.NewVolume`)))
    (:`NewEnumerator2`
      (setmembers `/Game/Menu/S_AudioMix` :`StructRef` (`/Game/BP_SaveSTP.AudioMixer` (`self.UserSettings`)) :`Effects` (`local.NewVolume`)))))