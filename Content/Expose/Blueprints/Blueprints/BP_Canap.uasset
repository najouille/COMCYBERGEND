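; BP_Canap is a Horror Engine prop that appears only as a collidable object once the player has seen a clue.
; Tick polls the player character, enabling actor collision while IndiceVu is above zero, then destroying the actor if Glitch is also set.
; Box overlaps set and clear the character's IsOverlapping flag, with setting gated on UseableValid.
; The construction script applies default horror-event, mesh and inspection settings.
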(event `self.ReceiveTick`
  (params (DeltaSeconds :type "Float (single-precision)"))
  (bind _ashorror_engine_character (cast `/Game/HorrorEngine/Blueprints/Core/HorrorEngineCharacter` (`GameplayStatics.GetPlayerCharacter` 0)))
  (if (> (`/Game/HorrorEngine/Blueprints/Core/HorrorEngineCharacter.IndiceVu` _ashorror_engine_character) 0)
    (`self.SetActorEnableCollision` true)
    (if (`/Game/HorrorEngine/Blueprints/Core/HorrorEngineCharacter.Glitch` _ashorror_engine_character)
      (`self.K2_DestroyActor`))
    (else
      (`self.SetActorEnableCollision` false))))

(event `self.Box.OnComponentBeginOverlap`
  (params (OverlappedComponent :type "PrimitiveComponent Object Reference") (OtherActor :type "Actor Object Reference") (OtherComp :type "PrimitiveComponent Object Reference") (OtherBodyIndex :type Integer) (bFromSweep :type Boolean) (SweepResult :type "HitResult Structure (by ref)"))
  (bind _asmaster (`/Game/HorrorEngine/Blueprints/Core/HorrorEngineFunctions.GetPlayer`))
  (if (`/Game/HorrorEngine/HorrorEngine.UseableValid` _asmaster)
    (bind _ashorror_engine_character (cast `/Game/HorrorEngine/Blueprints/Core/HorrorEngineCharacter` OtherActor))
    (set `/Game/HorrorEngine/Blueprints/Core/HorrorEngineCharacter.isOverlapping` true _ashorror_engine_character)))

(event `self.Box.OnComponentEndOverlap`
  (params (OverlappedComponent :type "PrimitiveComponent Object Reference") (OtherActor :type "Actor Object Reference") (OtherComp :type "PrimitiveComponent Object Reference") (OtherBodyIndex :type Integer))
  (bind _ashorror_engine_character (cast `/Game/HorrorEngine/Blueprints/Core/HorrorEngineCharacter` OtherActor))
  (set `/Game/HorrorEngine/Blueprints/Core/HorrorEngineCharacter.isOverlapping` false _ashorror_engine_character))

(fn `UserConstructionScript`
  (`parent.UserConstructionScript`)
  (`/Game/HorrorEngine/Blueprints/Core/HorrorEngineMacros.HM_DefaultConstructions` (`self.Horror Events`))
  (`/Game/HorrorEngine/Blueprints/Core/HorrorEngineFunctions.SetMesh` (`self.StaticMesh`) (`self.Mesh Settings`))
  (`self.SetInspection` (`self.Inspection Settings`)))