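; BP_Phone is a phone actor, set up for inspection, that becomes available once the player has seen more than three clues.
; Every Tick it reads IndiceVu on the HorrorEngineCharacter and toggles collision and custom-depth rendering to match.
; The construction script runs the parent's, then applies horror event defaults, mesh and inspection settings.
; A Glitch-based destroy branch is present but never runs.
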(event `self.ReceiveTick`
  (params (DeltaSeconds :type "Float (single-precision)"))
  (bind _ashorror_engine_character (cast `/Game/HorrorEngine/Blueprints/Core/HorrorEngineCharacter` (`GameplayStatics.GetPlayerCharacter` 0)))
  (if (> (`/Game/HorrorEngine/Blueprints/Core/HorrorEngineCharacter.IndiceVu` _ashorror_engine_character) 3)
    (`self.SetActorEnableCollision` true)
    (`PrimitiveComponent.SetRenderCustomDepth` (`self.StaticMesh`) true)
    (else
      (`self.SetActorEnableCollision` false)
      (`PrimitiveComponent.SetRenderCustomDepth` (`self.StaticMesh`) false))))

(fn `UserConstructionScript`
  (`parent.UserConstructionScript`)
  (`/Game/HorrorEngine/Blueprints/Core/HorrorEngineMacros.HM_DefaultConstructions` (`self.Horror Events`))
  (`/Game/HorrorEngine/Blueprints/Core/HorrorEngineFunctions.SetMesh` null (`self.Mesh Settings`))
  (`self.SetInspection` (`self.Inspection Settings`)))