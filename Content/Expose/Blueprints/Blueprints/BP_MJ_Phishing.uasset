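; BP_MJ_Phishing is an interactable actor for the HorrorEngineCharacter that stays inactive until the player's IndiceVu count is above zero.
; Tick toggles actor collision from that count and, while enabled, destroys the actor if the last overlapping character's Glitch flag is set.
; Box overlap events set the character's IsOverlapping flag, show or hide the E component as a prompt, and print debug messages.
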(event `self.ReceiveTick`
  (params (DeltaSeconds :type "Float (single-precision)"))
  (bind _ashorror_engine_character (cast `/Game/HorrorEngine/Blueprints/Core/HorrorEngineCharacter` (`GameplayStatics.GetPlayerCharacter` 0)))
  (if (> (`/Game/HorrorEngine/Blueprints/Core/HorrorEngineCharacter.IndiceVu` _ashorror_engine_character) 0)
    (`self.SetActorEnableCollision` true)
    (`/Engine/EditorBlueprintResources/StandardMacros.IsValid` (stale `self.Box.OnComponentBeginOverlap` OtherActor)
      (:`Is Valid`
        (if (`/Game/HorrorEngine/Blueprints/Core/HorrorEngineCharacter.Glitch` (stale `self.Box.OnComponentBeginOverlap` _ashorror_engine_character))
          (`self.K2_DestroyActor`))))
    (else
      (`self.SetActorEnableCollision` false))))

(event `self.Box.OnComponentBeginOverlap`
  (params (OverlappedComponent :type "PrimitiveComponent Object Reference") (OtherActor :type "Actor Object Reference") (OtherComp :type "PrimitiveComponent Object Reference") (OtherBodyIndex :type Integer) (bFromSweep :type Boolean) (SweepResult :type "HitResult Structure (by ref)"))
  (bind _ashorror_engine_character (cast `/Game/HorrorEngine/Blueprints/Core/HorrorEngineCharacter` OtherActor))
  (set `/Game/HorrorEngine/Blueprints/Core/HorrorEngineCharacter.isOverlapping` true _ashorror_engine_character)
  (`KismetSystemLibrary.PrintString` "overlapping")
  (`SceneComponent.SetVisibility` (`self.E`) true false))

(event `self.Box.OnComponentEndOverlap`
  (params (OverlappedComponent :type "PrimitiveComponent Object Reference") (OtherActor :type "Actor Object Reference") (OtherComp :type "PrimitiveComponent Object Reference") (OtherBodyIndex :type Integer))
  (set `/Game/HorrorEngine/Blueprints/Core/HorrorEngineCharacter.isOverlapping` false (stale `self.Box.OnComponentBeginOverlap` _ashorror_engine_character))
  (`KismetSystemLibrary.PrintString` "no overlap")
  (`SceneComponent.SetVisibility` (`self.E`) false false))

(fn `UserConstructionScript`)