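; A one-shot subtitle trigger volume that destroys itself after use.
; The first overlap of its collision component calls GetSousTitres on the first SousTitres entry, waits that entry's duration, then removes the returned widget and destroys the actor.
; End overlap does the same cleanup only if IsOver is set.
; Both events cast player 0's pawn to HorrorEngineCharacter without checking the overlapping actor.
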(event `self.CollisionComponent.OnComponentBeginOverlap`
  (params (OverlappedComponent :type "PrimitiveComponent Object Reference") (OtherActor :type "Actor Object Reference") (OtherComp :type "PrimitiveComponent Object Reference") (OtherBodyIndex :type Integer) (bFromSweep :type Boolean) (SweepResult :type "HitResult Structure (by ref)"))
  (cast `/Game/HorrorEngine/Blueprints/Core/HorrorEngineCharacter` (`GameplayStatics.GetPlayerCharacter` 0))
  (`/Engine/EditorBlueprintResources/StandardMacros.DoOnce` false
    (:`Completed`
      (set `self.isOver` false)
      (bind (_widget_ref `_durée`) (`/Game/Expose/Blueprints/Blueprints/ExposeFunctions.GetSousTitres` (`|GetArrayItem` (`self.Sous-Titres`))))
      (`KismetSystemLibrary.Delay` `_durée`)
      (set `self.isOver` true)
      (`Widget.RemoveFromParent` _widget_ref)
      (`self.K2_DestroyActor` :!label _label))))

(event `self.CollisionComponent.OnComponentEndOverlap`
  (params (OverlappedComponent :type "PrimitiveComponent Object Reference") (OtherActor :type "Actor Object Reference") (OtherComp :type "PrimitiveComponent Object Reference") (OtherBodyIndex :type Integer))
  (cast `/Game/HorrorEngine/Blueprints/Core/HorrorEngineCharacter` (`GameplayStatics.GetPlayerCharacter` 0))
  (if (`self.isOver`)
    (`Widget.RemoveFromParent` (stale `self.CollisionComponent.OnComponentBeginOverlap` _widget_ref))
    (goto _label)))

(fn `UserConstructionScript`)