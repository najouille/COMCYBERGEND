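; Trigger box that shows a one-time tutorial notification when the player's HorrorEngineCharacter enters it.
; BeginPlay pre-creates the Tutoriel_Notifications widget with its text; the first overlap gets a subtitle widget and duration from the first SousTitres entry.
; The notification animation plays for that duration minus one second, then jumps to a late start time for its final second.
; Both widgets are then removed, and again on exit once completed.
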(event `self.ReceiveBeginPlay`
  (bind _returnvalue (`|CreateWidget` "/Game/Expose/Blueprints/Widgets/Tutoriel/Tutoriel_Notifications.Tutoriel_Notifications_C"))
  (bind _output_get (set `self.NotifWidgetRef` _returnvalue))
  (`TextBlock.SetText` (`/Game/Expose/Blueprints/Widgets/Tutoriel/Tutoriel_Notifications.TextBlock_39` _output_get) (`self.Texte_Notif`)))

(event `self.Box.OnComponentBeginOverlap`
  (params (OverlappedComponent :type "PrimitiveComponent Object Reference") (OtherActor :type "Actor Object Reference") (OtherComp :type "PrimitiveComponent Object Reference") (OtherBodyIndex :type Integer) (bFromSweep :type Boolean) (SweepResult :type "HitResult Structure (by ref)"))
  (bind _notifwidgetref (`self.NotifWidgetRef`))
  (bind _notifwidgetref_2 (`self.NotifWidgetRef`))
  (bind _notifications (`/Game/Expose/Blueprints/Widgets/Tutoriel/Tutoriel_Notifications.Notifications` _notifwidgetref))
  (cast `/Game/HorrorEngine/Blueprints/Core/HorrorEngineCharacter` (`GameplayStatics.GetPlayerCharacter` 0))
  (`/Engine/EditorBlueprintResources/StandardMacros.DoOnce` false
    (:`Completed`
      (bind (_widget_ref `_durée`) (`/Game/Expose/Blueprints/Blueprints/ExposeFunctions.GetSousTitres` (`|GetArrayItem` (`self.Sous-Titres`))))
      (set `self.Widget Ref` _widget_ref)
      (set `self.Durée` `_durée`)
      (`self.Duree`)
      (`UserWidget.AddToViewport` _notifwidgetref_2 0)
      (`UserWidget.PlayAnimation` _notifwidgetref_2 (`/Game/Expose/Blueprints/Widgets/Tutoriel/Tutoriel_Notifications.Notifications` _notifwidgetref_2) 0.0 1 "Forward" 1.0 false)
      (`KismetSystemLibrary.Delay` (`self.DuréeNotif`))
      (`UserWidget.StopAnimation` _notifwidgetref _notifications)
      (`UserWidget.PlayAnimation` _notifwidgetref _notifications 9.0 1 "Forward" 1.0 false)
      (`KismetSystemLibrary.Delay` 1.0)
      (set `self.isCompleted` true)
      (`Widget.RemoveFromParent` (`self.NotifWidgetRef`))
      (`Widget.RemoveFromParent` (`self.Widget Ref`)))))

(event `self.Box.OnComponentEndOverlap`
  (params (OverlappedComponent :type "PrimitiveComponent Object Reference") (OtherActor :type "Actor Object Reference") (OtherComp :type "PrimitiveComponent Object Reference") (OtherBodyIndex :type Integer))
  (cast `/Game/HorrorEngine/Blueprints/Core/HorrorEngineCharacter` (`GameplayStatics.GetPlayerCharacter` 0))
  (if (`self.isCompleted`)
    (`Widget.RemoveFromParent` (`self.Widget Ref`))
    (`Widget.RemoveFromParent` (`self.NotifWidgetRef`))))

(fn `Duree`
  (set `self.DuréeNotif` (- (`self.Durée`) 1.0))
  (return))

(fn `UserConstructionScript`)