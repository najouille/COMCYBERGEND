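; Trigger volume that shows a one-time tutorial notification when an overlap with its box ends.
; BeginPlay creates the Tutoriel_Notifications widget and sets its text from TexteNotif.
; On end overlap, a DoOnce, gated by a BP_WCW_Character cast on player 0 rather than the overlapping actor, displays and animates it.
; Delays derived from DuréeAnimation time an animation restart at a fixed offset, then the widget's removal.
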(event `self.ReceiveBeginPlay`
  (bind _returnvalue (`|CreateWidget` "/Game/Expose/Blueprints/Widgets/Tutoriel/Tutoriel_Notifications.Tutoriel_Notifications_C"))
  (bind _output_get (set `self.NotifWidgetRef` _returnvalue))
  (`TextBlock.SetText` (`/Game/Expose/Blueprints/Widgets/Tutoriel/Tutoriel_Notifications.TextBlock_39` _output_get) (`self.Texte_Notif`)))

(event `self.Box.OnComponentBeginOverlap`
  (params (OverlappedComponent :type "PrimitiveComponent Object Reference") (OtherActor :type "Actor Object Reference") (OtherComp :type "PrimitiveComponent Object Reference") (OtherBodyIndex :type Integer) (bFromSweep :type Boolean) (SweepResult :type "HitResult Structure (by ref)")))

(event `self.Box.OnComponentEndOverlap`
  (params (OverlappedComponent :type "PrimitiveComponent Object Reference") (OtherActor :type "Actor Object Reference") (OtherComp :type "PrimitiveComponent Object Reference") (OtherBodyIndex :type Integer))
  (bind _notifwidgetref (`self.NotifWidgetRef`))
  (bind _notifwidgetref_2 (`self.NotifWidgetRef`))
  (bind _notifications (`/Game/Expose/Blueprints/Widgets/Tutoriel/Tutoriel_Notifications.Notifications` _notifwidgetref_2))
  (cast `/Game/WorkingComputerAndWifi/WCW_Blueprints/BP_WCW_Character` (`GameplayStatics.GetPlayerCharacter` 0))
  (`/Engine/EditorBlueprintResources/StandardMacros.DoOnce` false
    (:`Completed`
      (`self.Duree`)
      (`UserWidget.AddToViewport` _notifwidgetref 0)
      (`UserWidget.PlayAnimation` _notifwidgetref (`/Game/Expose/Blueprints/Widgets/Tutoriel/Tutoriel_Notifications.Notifications` _notifwidgetref) 0.0 1 "Forward" 1.0 false)
      (`KismetSystemLibrary.Delay` (`self.DuréeNotif`))
      (`UserWidget.StopAnimation` _notifwidgetref_2 _notifications)
      (`UserWidget.PlayAnimation` _notifwidgetref_2 _notifications 9.0 1 "Forward" 1.0 false)
      (`KismetSystemLibrary.Delay` (- (`self.DuréeNotif`) -1.0))
      (set `self.isCompleted` true)
      (`Widget.RemoveFromParent` (`self.NotifWidgetRef`)))))

(fn `Duree`
  (set `self.DuréeNotif` (- (`self.DuréeAnimation`) 1.0))
  (return))

(fn `UserConstructionScript`)